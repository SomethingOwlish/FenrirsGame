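; BP_WolfPlayer is a player Blueprint that toggles the hero between human and wolf forms.
; The Switch input action reads the HeroType enum as a boolean to choose the branch, then sets the new type.
; Each branch swaps the Mesh component's skeletal mesh, animation class and first material slot to match that form.
; BeginPlay, overlap, Tick and the construction script contain no logic.
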(event `InputAction|Switch` :consume false :paused true
  (params (Key :type "Key Structure"))
  (bind _mesh (`self.Mesh`))
  (:`Pressed`
    (if (`KismetMathLibrary.Conv_IntToBool` (`KismetMathLibrary.Conv_ByteToInt` (`self.HeroType`)))
      (set `self.HeroType` "Wolf")
      (`SkinnedMeshComponent.SetSkinnedAssetAndUpdate` _mesh "/Game/AnimalVarietyPack/Wolf/Meshes/SK_Wolf.SK_Wolf" false)
      (`SkeletalMeshComponent.SetAnimInstanceClass` _mesh "/Game/Animation/BP_AnimWolf.BP_AnimWolf_C")
      (`PrimitiveComponent.SetMaterial` _mesh 0 "/Game/AnimalVarietyPack/Wolf/Materials/M_WolfFurArctic.M_WolfFurArctic")
      (else
        (set `self.HeroType` "Human")
        (`SkinnedMeshComponent.SetSkinnedAssetAndUpdate` _mesh "/Game/ActorCore_Sample_Motions/Dummy_Female/Dummy_Female.Dummy_Female" false)
        (`SkeletalMeshComponent.SetAnimInstanceClass` _mesh "/Game/Animation/BP_Human.BP_Human_C")
        (`PrimitiveComponent.SetMaterial` _mesh 0 "/Game/Scanned3DPeoplePack/RP_Character/rp_sophia_rigged_003_ue4/Materials/rp_sophia_rigged_003_mat.rp_sophia_rigged_003_mat")))))

(event `self.ReceiveTick`
  (params (DeltaSeconds :type "Float (single-precision)")))

(fn `UserConstructionScript`)